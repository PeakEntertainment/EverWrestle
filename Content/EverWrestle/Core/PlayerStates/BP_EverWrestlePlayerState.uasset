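; Player state for EverWrestle that tracks whether its player is talking in voice chat.
; On BeginPlay it caches the EverWrestle game state and binds to the game player controller's voice chat state change event, which updates the talking flag.
; The flag's RepNotify passes this player and the new value to the cached game state's multicast talking-state change.
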(event Custom|OnPlayerVoiceStateChanged
  (params (IsTalking :type Boolean))
  ;[0.15 0.15 1 0.502] Setup VoiceChat Delegates
  (Variables|Default|SetbIsTalking IsTalking))

(event EventBeginPlay
  ;[0.15 0.15 1 0.502] Setup VoiceChat Delegates
  (bind _asbp_ever_wrestle_game_state (Utilities|Casting|CastToBP_EverWrestleGameState (Game|GetGameState)))
  (Variables|Default|SetCachedGameState _asbp_ever_wrestle_game_state)
  (bind _asbp_game_player_controller (Utilities|Casting|CastToBP_GamePlayerController (Game|GetPlayerController)))
  (EventDispatchers|BindEventtoOnVoicechatStateChanged _asbp_game_player_controller (delegate Custom|OnPlayerVoiceStateChanged)))

(fn ConstructionScript)

(fn OnRepBIsTalking
  (Class|EverWrestleGameState|MulticastChangeTalkingState (Variables|Default|GetCachedGameState) self (Variables|Default|GetbIsTalking)))