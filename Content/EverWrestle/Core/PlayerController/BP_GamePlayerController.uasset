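; Player controller for EverWrestle that manages match start-up and forwards player input to the possessed character.
; On local possession it locks movement, retries caching game state, character and HUD, starts music, reports loaded to the server, and frees movement once all players are ready.
; Enhanced Input drives movement, camera, grab, punch, checkpoint reset, pause toggling and push-to-talk or radio voice chat.
; A client event briefly mutes voice through a sound mix.
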(event Custom|Server_PlayerLoaded
  ;[0.15 0.15 1 0.502] Send the notification to the server that the player has loaded
  (bind _asbp_ever_wrestle_game_mode (Utilities|Casting|CastToBP_EverWrestleGameMode (Game|GetGameMode)))
  (Class|EverWrestleGameMode|OnPlayerReady _asbp_ever_wrestle_game_mode self))

(event Custom|ToggleInput
  (params (bIgnoreInputs :type Boolean))
  ;[0.02624 0.15 0 0.502] Switch between the Game and Pause Menu
  (Utilities|FlowControl|Sequence
    (:then_0
      (Input|SetIgnoreMoveInput bIgnoreInputs))
    (:then_1
      (Input|SetIgnoreLookInput bIgnoreInputs))))

(event Custom|SwitchGameAndPause
  ;[0.02624 0.15 0 0.502] Switch between the Game and Pause Menu
  (bind _bignoreinputs (Default|SwitchGameandPause (Variables|Default|GetCachedGameHUD)))
  (CallFunction|ToggleInput _bignoreinputs))

(event Custom|SetPlayerFree
  ;[0.15 0.15 1 0.502] Set the Cached Variables and set the player free when everyone is ready
  (Input|SetIgnoreMoveInput false))

(event Input|EnhancedActionEvents|EnhancedInputActionIA_ResetToCheckpoint
  (params (ActionValue :type Boolean) (ElapsedSeconds :type Float%20%28double-precision%29) (TriggeredSeconds :type Float%20%28double-precision%29) (InputAction :type Input%20Action%20Object%20Reference :default "/Game/EverWrestle/Core/Input/GameMapping/InputActions/IA_ResetToCheckpoint.IA_ResetToCheckpoint"))
  ;[0.15 0.15 1 0.502] Reset the player to the last collected checkpoint
  (Class|EverWrestleCharacterInterface|SetRagdolled (Variables|Default|GetCachedCharacter) false)
  (Class|EverWrestleCharacter|ResettoLastCheckpoint (Variables|Default|GetCachedCharacter)))

(event Input|EnhancedActionEvents|EnhancedInputActionIA_Pause
  (params (ActionValue :type Boolean) (ElapsedSeconds :type Float%20%28double-precision%29) (TriggeredSeconds :type Float%20%28double-precision%29) (InputAction :type Input%20Action%20Object%20Reference :default "/Game/EverWrestle/Core/Input/GameMapping/InputActions/IA_Pause.IA_Pause"))
  ;[0.02624 0.15 0 0.502] Switch between the Game and Pause Menu
  (:Started
    (CallFunction|SwitchGameandPause)))

(event Input|EnhancedActionEvents|EnhancedInputActionIA_Move
  (params (ActionValue :type Vector%202D%20Structure) (ElapsedSeconds :type Float%20%28double-precision%29) (TriggeredSeconds :type Float%20%28double-precision%29) (InputAction :type Input%20Action%20Object%20Reference :default "/Game/EverWrestle/Core/Input/GameMapping/InputActions/IA_Move.IA_Move"))
  ;[0.15 0.15 1 0.502] Movement
  (Class|EverWrestleCharacter|DoMove (Variables|Default|GetCachedCharacter) ActionValue))

(event Input|EnhancedActionEvents|EnhancedInputActionIA_Look
  (params (ActionValue :type Vector%202D%20Structure) (ElapsedSeconds :type Float%20%28double-precision%29) (TriggeredSeconds :type Float%20%28double-precision%29) (InputAction :type Input%20Action%20Object%20Reference :default "/Game/EverWrestle/Core/Input/GameMapping/InputActions/IA_Look.IA_Look"))
  ;[0.15 0.15 1 0.502] Camera Movement
  (Class|EverWrestleCharacter|DoLook (Variables|Default|GetCachedCharacter) ActionValue))

(event Input|EnhancedActionEvents|EnhancedInputActionIA_Jump
  (params (ActionValue :type Boolean) (ElapsedSeconds :type Float%20%28double-precision%29) (TriggeredSeconds :type Float%20%28double-precision%29) (InputAction :type Input%20Action%20Object%20Reference :default "/Game/EverWrestle/Core/Input/GameMapping/InputActions/IA_Jump.IA_Jump"))
  ;[0.15 0.15 1 0.502] Movement
  (:Triggered
    (Class|EverWrestleCharacter|DoJumpStart (Variables|Default|GetCachedCharacter)))
  (:Started
    (if (AI|Components|NavMovement|IsFalling (Variables|/Script/Engine.Character|GetCharacterMovement (Variables|Default|GetCachedCharacter)))
      (Default|ServerMantleEvent (Variables|Default|GetCachedCharacter))))
  (:Completed
    (Class|EverWrestleCharacter|DoJumpEnd (Variables|Default|GetCachedCharacter))))

(event Input|EnhancedActionEvents|EnhancedInputActionIA_Grab
  (params (ActionValue :type Boolean) (ElapsedSeconds :type Float%20%28double-precision%29) (TriggeredSeconds :type Float%20%28double-precision%29) (InputAction :type Input%20Action%20Object%20Reference :default "/Game/EverWrestle/Core/Input/GameMapping/InputActions/IA_Grab.IA_Grab"))
  (bind _cachedcharacter (Variables|Default|GetCachedCharacter))
  ;[0.15 0.15 1 0.502] Interactions
  (:Started
    (Default|HandleGrabPressed _cachedcharacter))
  (:Completed
    (Default|HandleGrabReleased _cachedcharacter)))

(event Input|EnhancedActionEvents|EnhancedInputActionIA_Punch
  (params (ActionValue :type Boolean) (ElapsedSeconds :type Float%20%28double-precision%29) (TriggeredSeconds :type Float%20%28double-precision%29) (InputAction :type Input%20Action%20Object%20Reference :default "/Game/EverWrestle/Core/Input/GameMapping/InputActions/IA_Punch.IA_Punch"))
  ;[0.15 0.15 1 0.502] Interactions
  (:Started
    (Default|ServerPunch (Variables|Default|GetCachedCharacter))))

(event Input|EnhancedActionEvents|EnhancedInputActionIA_PushToTalk
  (params (ActionValue :type Boolean) (ElapsedSeconds :type Float%20%28double-precision%29) (TriggeredSeconds :type Float%20%28double-precision%29) (InputAction :type Input%20Action%20Object%20Reference :default "/Game/EverWrestle/Core/Input/GameMapping/InputActions/IA_PushToTalk.IA_PushToTalk"))
  (bind _cachedcharacter (Variables|Default|GetCachedCharacter))
  ;[1 0.07227 0 0.502] Voicechat
  (:Started
    (Default|StartTalking _cachedcharacter "NewEnumerator1")
    (Default|CallOnVoicechatStateChanged true))
  (:Completed
    (Default|StopTalking _cachedcharacter)
    (Default|CallOnVoicechatStateChanged false)))

(event Input|EnhancedActionEvents|EnhancedInputActionIA_RadioTalk
  (params (ActionValue :type Boolean) (ElapsedSeconds :type Float%20%28double-precision%29) (TriggeredSeconds :type Float%20%28double-precision%29) (InputAction :type Input%20Action%20Object%20Reference :default "/Game/EverWrestle/Core/Input/GameMapping/InputActions/IA_RadioTalk.IA_RadioTalk"))
  (bind _cachedcharacter (Variables|Default|GetCachedCharacter))
  ;[1 0.07227 0 0.502] Voicechat
  (:Started
    (Default|StartTalking _cachedcharacter "NewEnumerator2")
    (Default|CallOnVoicechatStateChanged true))
  (:Completed
    (Default|StopTalking _cachedcharacter)
    (Default|CallOnVoicechatStateChanged false)))

(event EventOnControllerPossessed
  ;[0.15 0.15 1 0.502] Set the Cached Variables and set the player free when everyone is ready
  (if (Pawn|IsLocalController) :!label _label
    (Utilities|IsValid (Pawn|GetControlledPawn)
      (:Is%20Valid
        (Input|SetIgnoreMoveInput true)
        (bind _asbp_ever_wrestle_game_state (Utilities|Casting|CastToBP_EverWrestleGameState (Game|GetGameState) :!label _label_2)
          (:then
            (EventDispatchers|BindEventtoOnAllPlayersReadyDelegate _asbp_ever_wrestle_game_state (delegate Custom|SetPlayerFree))
            (bind _returnvalue (Class|EverWrestleGameState|GetIsGameReady _asbp_ever_wrestle_game_state))
            (if _returnvalue
              (CallFunction|SetPlayerFree))
            (bind _asbp_ever_wrestle_character (Utilities|Casting|CastToBP_EverWrestleCharacter (Pawn|GetControlledPawn)))
            (Variables|Default|SetCachedCharacter _asbp_ever_wrestle_character)
            (bind _asbp_game_hud (Utilities|Casting|CastToBP_GameHUD (HUD|GetHUD) :!label _label_3)
              (:then
                (bind _output_get (Variables|Default|SetCachedGameHUD _asbp_game_hud))
                (bind _aswbp_game_hud (Utilities|Casting|CastToWBP_GameHUD (Variables|/Script/EverWrestle.EverWrestleHUD|GetCurrentGameHUD _output_get) :!label _label_4)
                  (:then
                    (Variables|Default|SetCachedGameWidget _aswbp_game_hud)
                    (Utilities|FlowControl|DoOnce false
                      (:Completed
                        (bind _returnvalue_2 (Audio|SpawnSound2D "/Game/EverWrestle/Core/Sounds/Everwrestle_OST_V4.Everwrestle_OST_V4" 1.0 1.0 0.0 0))
                        (Audio|Components|Audio|FadeIn _returnvalue_2 5.0 1.0 0.0 "Linear" :!class /Script/Engine.AudioComponent)
                        (CallFunction|ServerPlayerLoaded))))
                  (:CastFailed
                    (Utilities|FlowControl|RetriggerableDelay 0.2)
                    (goto _label_4))))
              (:CastFailed
                (Utilities|FlowControl|RetriggerableDelay 0.2)
                (goto _label_3))))
          (:CastFailed
            (Utilities|FlowControl|RetriggerableDelay 0.2)
            (goto _label_2))))
      (:Is%20Not%20Valid
        (goto _label)))))

(event Custom|Client_ToggleVoiceAtStart
  (if (Pawn|IsLocalPlayerController)
    (Class|GameplayStatics|SetBaseSoundMix "/Game/EverWrestle/Core/ProximityChat/SCM_MuteVoice.SCM_MuteVoice")
    (Utilities|Time|SetTimerbyEvent (delegate Custom|UnMuteVoice) 1.0)))

(event Custom|UnMuteVoice
  (Class|GameplayStatics|SetBaseSoundMix "/Game/EverWrestle/Core/Sounds/SCM_MainSoundMix.SCM_MainSoundMix"))

(fn ConstructionScript)