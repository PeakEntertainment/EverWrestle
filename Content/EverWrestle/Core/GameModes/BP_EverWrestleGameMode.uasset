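; Game mode for EverWrestle that initializes voice chat whenever a player logs in or is started as a new player.
; Both events run duplicated logic, first telling the player's controller to toggle voice on the client.
; They poll with short retriggerable delays until pawns are possessed, then multicast VOIP setup on every player's character, re-initializing existing players too.
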(event EventHandleStartingNewPlayer
  (params (NewPlayer :type Player%20Controller%20Object%20Reference))
  ;[0.15 0.15 1 0.502] Initialize VoiceChat
  (|CallParentFunction NewPlayer)
  (bind _asbp_game_player_controller (Utilities|Casting|CastToBP_GamePlayerController NewPlayer))
  (Default|ClientToggleVoiceatStart _asbp_game_player_controller)
  (Utilities|IsValid (Pawn|GetControlledPawn _asbp_game_player_controller) :!label _label
    (:Is%20Valid
      (for _array_element (Variables|/Script/Engine.GameStateBase|GetPlayerArray (Game|GetGameState))
        (Utilities|IsValid (Pawn|GetControlledPawn (Game|GetPlayerController _array_element)) :!label _label_2
          (:Is%20Valid
            (bind _asbp_ever_wrestle_character (Utilities|Casting|CastToBP_EverWrestleCharacter (Pawn|GetControlledPawn (Game|GetPlayerController _array_element))))
            (Default|MulticastInitVOIP _asbp_ever_wrestle_character))
          (:Is%20Not%20Valid
            (Utilities|FlowControl|RetriggerableDelay 0.2)
            (goto _label_2)))))
    (:Is%20Not%20Valid
      (Utilities|FlowControl|RetriggerableDelay 0.2)
      (goto _label))))

(event EventPostLogin
  (params (NewPlayer :type Player%20Controller%20Object%20Reference))
  ;[0.15 0.15 1 0.502] Initialize VoiceChat
  (bind _asbp_game_player_controller (Utilities|Casting|CastToBP_GamePlayerController NewPlayer))
  (Default|ClientToggleVoiceatStart _asbp_game_player_controller)
  (Utilities|IsValid (Pawn|GetControlledPawn _asbp_game_player_controller) :!label _label
    (:Is%20Valid
      (for _array_element (Variables|/Script/Engine.GameStateBase|GetPlayerArray (Game|GetGameState))
        (Utilities|IsValid (Pawn|GetControlledPawn (Game|GetPlayerController _array_element)) :!label _label_2
          (:Is%20Valid
            (bind _asbp_ever_wrestle_character (Utilities|Casting|CastToBP_EverWrestleCharacter (Pawn|GetControlledPawn (Game|GetPlayerController _array_element))))
            (Default|MulticastInitVOIP _asbp_ever_wrestle_character))
          (:Is%20Not%20Valid
            (Utilities|FlowControl|RetriggerableDelay 0.2)
            (goto _label_2)))))
    (:Is%20Not%20Valid
      (Utilities|FlowControl|RetriggerableDelay 0.2)
      (goto _label))))

(fn ConstructionScript)