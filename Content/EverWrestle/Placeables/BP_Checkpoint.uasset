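; BP_Checkpoint is a placeable checkpoint that records which players have reached it.
; When an actor implementing the player interface overlaps it, the server adds that actor to a collected set, ignoring repeats, and sets it as that player's checkpoint.
; Once the set is at least as large as the game state's player array, an AllPlayersCollected flag is set.
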(event Custom|CheckIfAllPlayersCollected
  ;[0.15 0.15 1 0.502] Check if all Players collected the checkpoint -> Broadcast if yes
  (if (>= (Utilities|Set|Length (Variables|DeathzoneCommunication|GetPlayersCollected)) (Utilities|Array|Length (Variables|/Script/Engine.GameStateBase|GetPlayerArray (Game|GetGameState))))
    (Variables|DeathzoneCommunication|SetbAllPlayersCollected true)))

(event Collision|EventActorBeginOverlap
  (params (OtherActor :type Actor%20Object%20Reference))
  ;[0.15 0.15 1 0.502] Check if the Collision is valid and add the collided Actor to the Set
  (Utilities|ValidandImplementsPlayerInterface OtherActor
    (:Implements
      (if (not (Utilities|Set|Contains (Variables|DeathzoneCommunication|GetPlayersCollected) OtherActor))
        (Networking|SwitchHasAuthority
          (:Authority
            (Utilities|FlowControl|Sequence
              (:then_0
                (Utilities|Set|Add (Variables|DeathzoneCommunication|GetPlayersCollected) OtherActor)
                (CallFunction|CheckifAllPlayersCollected))
              (:then_1
                (Class|Checkpoint|ServerSetPlayerCheckPoint OtherActor)))))))))

(fn ConstructionScript)